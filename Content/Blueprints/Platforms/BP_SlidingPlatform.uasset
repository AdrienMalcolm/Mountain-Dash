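; BP_SlidingPlatform is a platform that slides back and forth endlessly between its Start0 and End points.
; On BeginPlay it sets the timeline play rate from SlidingTime and starts from either end according to Isgoingforward.
; The timeline's track lerps PlatformMesh's world location without sweep.
; Each time it finishes, a one-second delay precedes flipping the direction flag and playing or reversing the timeline.
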(event Custom|StartBackward
  (bind _newtrack_0 (Timeline|Sliding%20Timeline ReverseFromEnd)
    (:Update
      (Transformation|SetWorldLocation (Variables|Default|GetPlatformMesh) (Math|Vector|Lerp(Vector) (Transformation|GetWorldLocation (Variables|Default|GetStart_0)) (Transformation|GetWorldLocation (Variables|Default|GetEnd)) _newtrack_0) false false))
    (:Finished
      (Utilities|FlowControl|Delay 1.0)
      (if (Variables|Default|GetIsgoingforward)
        (Variables|Default|SetIsgoingforward false)
        (CallFunction|Backward)
        (else
          (Variables|Default|SetIsgoingforward true)
          (CallFunction|Forward))))))

(event Custom|Forward
  (bind _newtrack_0 (Timeline|Sliding%20Timeline Play)
    (:Update
      (Transformation|SetWorldLocation (Variables|Default|GetPlatformMesh) (Math|Vector|Lerp(Vector) (Transformation|GetWorldLocation (Variables|Default|GetStart_0)) (Transformation|GetWorldLocation (Variables|Default|GetEnd)) _newtrack_0) false false))
    (:Finished
      (Utilities|FlowControl|Delay 1.0)
      (if (Variables|Default|GetIsgoingforward)
        (Variables|Default|SetIsgoingforward false)
        (CallFunction|Backward)
        (else
          (Variables|Default|SetIsgoingforward true)
          (CallFunction|Forward))))))

(event Custom|StartForward
  (bind _newtrack_0 (Timeline|Sliding%20Timeline PlayFromStart)
    (:Update
      (Transformation|SetWorldLocation (Variables|Default|GetPlatformMesh) (Math|Vector|Lerp(Vector) (Transformation|GetWorldLocation (Variables|Default|GetStart_0)) (Transformation|GetWorldLocation (Variables|Default|GetEnd)) _newtrack_0) false false))
    (:Finished
      (Utilities|FlowControl|Delay 1.0)
      (if (Variables|Default|GetIsgoingforward)
        (Variables|Default|SetIsgoingforward false)
        (CallFunction|Backward)
        (else
          (Variables|Default|SetIsgoingforward true)
          (CallFunction|Forward))))))

(event Custom|Backward
  (bind _newtrack_0 (Timeline|Sliding%20Timeline Reverse)
    (:Update
      (Transformation|SetWorldLocation (Variables|Default|GetPlatformMesh) (Math|Vector|Lerp(Vector) (Transformation|GetWorldLocation (Variables|Default|GetStart_0)) (Transformation|GetWorldLocation (Variables|Default|GetEnd)) _newtrack_0) false false))
    (:Finished
      (Utilities|FlowControl|Delay 1.0)
      (if (Variables|Default|GetIsgoingforward)
        (Variables|Default|SetIsgoingforward false)
        (CallFunction|Backward)
        (else
          (Variables|Default|SetIsgoingforward true)
          (CallFunction|Forward))))))

(event EventBeginPlay
  (|CallParentFunction)
  (Components|Timeline|SetPlayRate (Variables|Default|GetSliding%20Timeline) (/ 1.0 (Variables|Default|GetSliding%20Time)))
  (if (Variables|Default|GetIsgoingforward)
    (CallFunction|StartForward)
    (else
      (CallFunction|StartBackward))))

(event Collision|EventActorBeginOverlap
  (params (OtherActor :type Actor%20Object%20Reference))
  (|CallParentFunction OtherActor) ; This node is disabled and will not be called.\nDrag off pins to build functionality.
)

(fn ConstructionScript
  (|CallParentFunction))